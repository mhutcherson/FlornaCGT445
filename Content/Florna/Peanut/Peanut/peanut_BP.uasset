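; Peanut is an animated character actor that idles, sits facing the player when approached, and explodes when hit.
; It starts on one of three idle loops at a random play rate.
; Its sphere overlap with Florna_Character runs a looping timer for yaw-only turning, then on exit clears it, plays a stand animation and resumes a random idle.
; Capsule hits from anything other than PlayerCharacter spawn a scaled explosion with sound and destroy it.
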(event `self.ReceiveBeginPlay`
  (switch `int` (`KismetMathLibrary.RandomIntegerInRange` 0 2)
    (:`0`
      (`SkeletalMeshComponent.PlayAnimation` (`self.Peanut`) "/Game/Florna/Peanut/Animations/peanut_idle.peanut_idle" true)
      (`SkeletalMeshComponent.SetPlayRate` (`self.Peanut`) (`KismetMathLibrary.RandomFloatInRange` (`self.PlayRateMin`) (`self.PlayRateMax`))))
    (:`1`
      (`SkeletalMeshComponent.PlayAnimation` (`self.Peanut`) "/Game/Florna/Peanut/Animations/peanut_idle_2.peanut_idle_2" true)
      (`SkeletalMeshComponent.SetPlayRate` (`self.Peanut`) (`KismetMathLibrary.RandomFloatInRange` (`self.PlayRateMin`) (`self.PlayRateMax`))))
    (:`2`
      (`SkeletalMeshComponent.PlayAnimation` (`self.Peanut`) "/Game/Florna/Peanut/Animations/peanut_idle_3.peanut_idle_3" true)
      (`SkeletalMeshComponent.SetPlayRate` (`self.Peanut`) (`KismetMathLibrary.RandomFloatInRange` (`self.PlayRateMin`) (`self.PlayRateMax`))))))

(event `self.Sphere.OnComponentBeginOverlap`
  (params (OverlappedComponent :type "PrimitiveComponent Object Reference") (OtherActor :type "Actor Object Reference") (OtherComp :type "PrimitiveComponent Object Reference") (OtherBodyIndex :type Integer) (bFromSweep :type Boolean) (SweepResult :type "HitResult Structure (by ref)"))
  (bind _asflorna_character (cast `/Game/Florna/Characters/Florna/Florna_Character` OtherActor))
  (bind _returnvalue (`KismetSystemLibrary.K2_SetTimerDelegate` (delegate `look at player`) 0.1 true))
  (`SkeletalMeshComponent.PlayAnimation` (`self.Peanut`) "/Game/Florna/Peanut/Animations/peanut_sit.peanut_sit" false))

(event `look at player`
  (bind (_returnvalue_roll _returnvalue_pitch _returnvalue_yaw) (`KismetMathLibrary.BreakRotator` (`KismetMathLibrary.FindLookAtRotation` (`self.K2_GetActorLocation`) (`self.K2_GetActorLocation` (stale `self.Sphere.OnComponentBeginOverlap` _asflorna_character)))))
  (`self.K2_SetActorRotation` (`KismetMathLibrary.MakeRotator` 0.0 0.0 (+ _returnvalue_yaw -90.0))))

(event `self.Sphere.OnComponentEndOverlap`
  (params (OverlappedComponent :type "PrimitiveComponent Object Reference") (OtherActor :type "Actor Object Reference") (OtherComp :type "PrimitiveComponent Object Reference") (OtherBodyIndex :type Integer))
  (cast `/Game/Florna/Characters/Florna/Florna_Character` OtherActor)
  (`KismetSystemLibrary.K2_ClearAndInvalidateTimerHandle` (stale `self.Sphere.OnComponentBeginOverlap` _returnvalue))
  (`SkeletalMeshComponent.PlayAnimation` (`self.Peanut`) "/Game/Florna/Peanut/Animations/peanut_stand.peanut_stand" false)
  (`KismetSystemLibrary.RetriggerableDelay` 0.95)
  (switch `int` (`KismetMathLibrary.RandomIntegerInRange` 0 2)
    (:`0`
      (`SkeletalMeshComponent.PlayAnimation` (`self.Peanut`) "/Game/Florna/Peanut/Animations/peanut_idle.peanut_idle" true)
      (`SkeletalMeshComponent.SetPlayRate` (`self.Peanut`) (`KismetMathLibrary.RandomFloatInRange` (`self.PlayRateMin`) (`self.PlayRateMax`))))
    (:`1`
      (`SkeletalMeshComponent.PlayAnimation` (`self.Peanut`) "/Game/Florna/Peanut/Animations/peanut_idle_2.peanut_idle_2" true)
      (`SkeletalMeshComponent.SetPlayRate` (`self.Peanut`) (`KismetMathLibrary.RandomFloatInRange` (`self.PlayRateMin`) (`self.PlayRateMax`))))
    (:`2`
      (`SkeletalMeshComponent.PlayAnimation` (`self.Peanut`) "/Game/Florna/Peanut/Animations/peanut_idle_3.peanut_idle_3" true)
      (`SkeletalMeshComponent.SetPlayRate` (`self.Peanut`) (`KismetMathLibrary.RandomFloatInRange` (`self.PlayRateMin`) (`self.PlayRateMax`))))))

(event `self.Capsule.OnComponentHit`
  (params (HitComponent :type "PrimitiveComponent Object Reference") (OtherActor :type "Actor Object Reference") (OtherComp :type "PrimitiveComponent Object Reference") (NormalImpulse :type "Vector Structure") (Hit :type "HitResult Structure (by ref)"))
  (cast `/Game/Needed_Stuff_For_Now/PlayerCharacter` OtherActor
    (:`CastFailed`
      (bind _returnvalue (`GameplayStatics.SpawnEmitterAtLocation` "/Game/StarterContent/Particles/P_Explosion.P_Explosion" (`SceneComponent.K2_GetComponentLocation` (`self.Capsule`))))
      (`SceneComponent.SetRelativeScale3D` _returnvalue (/ (`self.GetActorScale3D`) 2.5))
      (`GameplayStatics.SpawnSoundAttached` "/Game/StarterContent/Audio/Explosion02.Explosion02" (`self.Capsule`))
      (`self.K2_DestroyActor`))))

(fn `UserConstructionScript`)