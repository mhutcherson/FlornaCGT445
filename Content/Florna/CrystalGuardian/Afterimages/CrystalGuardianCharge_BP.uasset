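; Afterimage actor for the Crystal Guardian's charge, showing a short-lived, fading ghost mesh.
; On BeginPlay it applies the charge-phase mesh and computes a target a short distance along that mesh's right vector.
; Two sped-up timelines then run together: one teleports the actor toward the target, the other fades the material's Opacity parameter and destroys the actor when finished.
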(event `self.ReceiveBeginPlay`
  (bind _returnvalue (`SceneComponent.K2_GetComponentLocation` (`self.StaticMesh`)))
  (`StaticMeshComponent.SetStaticMesh` (`self.StaticMesh`) (`self.ChargePhase`))
  (set `self.DashInitialLocation` _returnvalue)
  (set `self.DashFinalLocation` (+ (* (`KismetMathLibrary.GetRightVector` (`SceneComponent.K2_GetComponentRotation` (`self.StaticMesh`))) 100.0) _returnvalue))
  (`TimelineComponent.SetPlayRate` (`self.Timeline_2`) 2.0)
  (`TimelineComponent.SetPlayRate` (`self.Timeline_0`) 2.0)
  (`|ExecutionSequence`
    (:`then_0`
      (bind (_direction _alpha) (`Timeline|Timeline_2` :!via `PlayFromStart`)
        (:`Update`
          (`self.K2_SetActorLocation` (`KismetMathLibrary.VLerp` (`self.DashInitialLocation`) (`self.DashFinalLocation`) _alpha) false true))))
    (:`then_1`
      (bind (_direction_2 _newtrack_0) (`Timeline|Timeline_0` :!via `PlayFromStart`)
        (:`Update`
          (`MeshComponent.SetScalarParameterValueOnMaterials` (`self.StaticMesh`) "Opacity" (`KismetMathLibrary.Lerp` 0.2 0.0 _newtrack_0)))
        (:`Finished`
          (`self.K2_DestroyActor`))))))

(fn `UserConstructionScript`)