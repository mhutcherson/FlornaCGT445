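; Projectile for the first boss's golem fist attack that hurts the player character, Florna, on contact.
; A sphere overlap with Florna subtracts a fixed amount from PlayerHP, calls Hurt and prints the remaining health.
; Any overlap, player or not, destroys the projectile and spawns a scaled-up explosion emitter at its location.
; The construction script makes the sphere ignore its instigator and itself while moving.
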(event `self.ReceiveBeginPlay`)

(event `self.Sphere.OnComponentBeginOverlap`
  (params (OverlappedComponent :type "PrimitiveComponent Object Reference") (OtherActor :type "Actor Object Reference") (OtherComp :type "PrimitiveComponent Object Reference") (OtherBodyIndex :type Integer) (bFromSweep :type Boolean) (SweepResult :type "HitResult Structure (by ref)"))
  (if (== (`GameplayStatics.GetObjectClass` OtherActor) "/Game/Florna/Florna/Florna.Florna_C")
    (bind _asflorna (cast `/Game/Florna/Florna/Florna` (`GameplayStatics.GetPlayerCharacter` 0)))
    (bind _output_get (set `/Game/Florna/Florna/Florna.PlayerHP` (- (`/Game/Florna/Florna/Florna.PlayerHP` _asflorna) 0.1) _asflorna))
    (`/Game/Florna/Florna/Florna.Hurt` _asflorna)
    (`self.K2_DestroyActor`)
    (`KismetSystemLibrary.PrintString` (`KismetStringLibrary.Conv_DoubleToString` _output_get) true true (struct :`R` 0.938721 :`G` 1.0 :`A` 1.0)))
  (`self.K2_DestroyActor`)
  (bind _returnvalue (`GameplayStatics.SpawnEmitterAtLocation` "/Game/StarterContent/Particles/P_Explosion2.P_Explosion2" (`self.K2_GetActorLocation`)))
  (`SceneComponent.SetWorldScale3D` _returnvalue (5.0 5.0 5.0)))

(fn `UserConstructionScript`
  (bind _sphere (`self.Sphere`))
  (`PrimitiveComponent.IgnoreActorWhenMoving` _sphere (`self.GetInstigator`) true)
  (`PrimitiveComponent.IgnoreActorWhenMoving` _sphere self true))