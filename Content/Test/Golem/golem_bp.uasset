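; Test golem enemy that lies as a ragdoll until the player enters its trigger box, then snaps up and slams.
; BeginPlay and sniper projectile hits switch the skeletal mesh to physics simulation.
; The trigger disables physics, moves the mesh to a reference scene root and plays the slam animation.
; A hitbox attached to the mesh's Hitbox socket has collision briefly during the slam, killing any player it overlaps.
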(event `self.ReceiveBeginPlay`
  (`SkeletalMeshComponent.PlayAnimation` (`self.SkeletalMesh`) "/Game/Test/Golem/golem_test_inert.golem_test_inert" false)
  (`KismetSystemLibrary.Delay` 0.1)
  (`PrimitiveComponent.SetSimulatePhysics` (`self.SkeletalMesh`) true)
  (`PrimitiveComponent.SetCollisionEnabled` (`self.Box1`) "NoCollision"))

(event `self.SkeletalMesh.OnComponentHit`
  (params (HitComponent :type "PrimitiveComponent Object Reference") (OtherActor :type "Actor Object Reference") (OtherComp :type "PrimitiveComponent Object Reference") (NormalImpulse :type "Vector Structure") (Hit :type "HitResult Structure (by ref)"))
  (cast `/Game/FirstPersonBP/Blueprints/Sniper_Projectile` OtherActor)
  (`PrimitiveComponent.SetSimulatePhysics` (`self.SkeletalMesh`) true))

(event `self.Box.OnComponentBeginOverlap`
  (params (OverlappedComponent :type "PrimitiveComponent Object Reference") (OtherActor :type "Actor Object Reference") (OtherComp :type "PrimitiveComponent Object Reference") (OtherBodyIndex :type Integer) (bFromSweep :type Boolean) (SweepResult :type "HitResult Structure (by ref)"))
  (bind _defaultsceneroot1 (`self.DefaultSceneRoot1`))
  (cast `/Game/PlayerCharacter` OtherActor)
  (`PrimitiveComponent.SetSimulatePhysics` (`self.SkeletalMesh`) false)
  (`SceneComponent.K2_SetRelativeLocationAndRotation` (`self.SkeletalMesh`) (`SceneComponent.K2_GetComponentLocation` _defaultsceneroot1) (`SceneComponent.K2_GetComponentRotation` _defaultsceneroot1) false false)
  (`SkeletalMeshComponent.PlayAnimation` (`self.SkeletalMesh`) "/Game/Test/Golem/golem_test_slam.golem_test_slam" false)
  (`KismetSystemLibrary.Delay` 0.05)
  (`PrimitiveComponent.SetCollisionEnabled` (`self.Box1`) "QueryAndPhysics")
  (`KismetSystemLibrary.Delay` 0.8)
  (`PrimitiveComponent.SetCollisionEnabled` (`self.Box1`) "NoCollision"))

(event `self.Box1.OnComponentBeginOverlap`
  (params (OverlappedComponent :type "PrimitiveComponent Object Reference") (OtherActor :type "Actor Object Reference") (OtherComp :type "PrimitiveComponent Object Reference") (OtherBodyIndex :type Integer) (bFromSweep :type Boolean) (SweepResult :type "HitResult Structure (by ref)"))
  (bind _asplayer_character (cast `/Game/PlayerCharacter` OtherActor))
  (`/Game/PlayerCharacter.PlayerDeath` _asplayer_character))

(fn `UserConstructionScript`
  (`SceneComponent.K2_AttachToComponent` (`self.Box1`) (`self.SkeletalMesh`) "Hitbox" "KeepRelative" "KeepRelative" "KeepRelative" true))