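; Test Blueprint for an "exploding ball" that endlessly animates a skeletal mesh morph target back and forth from BeginPlay.
; A timeline track drives the psphere2 morph weight on each update.
; When the timeline finishes, a FlipFlop alternates between custom backward and forward events, which reverse or play it to form a ping-pong loop.
; The construction script applies a gold metal material to the mesh.
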(event `self.ReceiveBeginPlay`
  (`SkeletalMeshComponent.SetMorphTarget` (`self.SkeletalMesh`) "None" 1.0 true)
  (bind (_direction _newtrack_0) (`Timeline|Timeline_0` :!label _label)
    (:`Update`
      (`SkeletalMeshComponent.SetMorphTarget` (`self.SkeletalMesh`) "psphere2" _newtrack_0 true))
    (:`Finished`
      (`/Engine/EditorBlueprintResources/StandardMacros.FlipFlop`
        (:`A`
          (`self.backward`))
        (:`B`
          (`self.forward`))))))

(event `forward`
  (goto _label))

(event `backward`
  (goto _label :!via `Reverse`))

(fn `UserConstructionScript`
  (`PrimitiveComponent.SetMaterial` (`self.SkeletalMesh`) 0 "/Game/StarterContent/Materials/M_Metal_Gold.M_Metal_Gold"))